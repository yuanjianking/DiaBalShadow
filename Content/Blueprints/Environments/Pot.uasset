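; Breakable decorative pot actor that swaps between an intact and a broken mesh.
; BeginPlay shows the intact mesh and hides the broken one, and the Brake function reverses their visibility.
; Cursor hover on the intact mesh applies a highlight overlay material, which is cleared when the cursor leaves.
; Nothing in this Blueprint calls Brake, and a WeaponActor class check is left unconnected.
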(event `self.ReceiveBeginPlay`
  (`SceneComponent.SetVisibility` (`self.SM_pot3`) true true)
  (`SceneComponent.SetVisibility` (`self.SM_pot1broken`) false true))

(event `self.SM_pot3.OnBeginCursorOver`
  (params (TouchedComponent :type "PrimitiveComponent Object Reference"))
  (`MeshComponent.SetOverlayMaterial` (`self.SM_pot3`) "/Game/InfinityBladeFireLands/Environments/Fire/Env_Fire_deco/Materials/M_Fire_Deco_Pots_HeightLight.M_Fire_Deco_Pots_HeightLight"))

(event `self.SM_pot3.OnEndCursorOver`
  (params (TouchedComponent :type "PrimitiveComponent Object Reference"))
  (`MeshComponent.SetOverlayMaterial` (`self.SM_pot3`) null))

(fn `Brake`
  (`SceneComponent.SetVisibility` (`self.SM_pot3`) false true)
  (`SceneComponent.SetVisibility` (`self.SM_pot1broken`) true true))

(fn `UserConstructionScript`)