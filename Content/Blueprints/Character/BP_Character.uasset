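; Player hero character using the Gameplay Ability System, with data tables supplying mesh, animation and passive effect for the GameInstance's chosen hero.
; Input drives camera zoom, melee and fireball abilities, a recover-buff toggle, toggled menu widgets and a gold-plus-Bear-spawn key.
; Weapon pickups enter the inventory, replace the socketed weapon and feed bonuses into stat getters.
; Experience counts down to each level-up, with the requirement scaling by level.
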(event `self.ReceiveBeginPlay`
  ;[1 1 1] Init
  (`self.InitCharacter`)
  (`self.CreateMenu`)
  (bind _returnvalue (`self.SetMaxCharacterExperience` (* (`self.GetCharacterLevel`) 100)))
  (`self.SetCharacterExperience` _returnvalue))

(event `Key|P`
  (params (Key :type "Key Structure"))
  (:`Pressed`
    (`self.AddGold` 15)
    (`|SpawnActorFromClass` "/Game/Blueprints/Enemy/Bear.Bear_C" (`self.GetTransform` (`GameplayStatics.GetPlayerPawn` 0)) "AdjustIfPossibleButAlwaysSpawn" "OverrideRootScale" null null)))

(event `Key|Five`
  (params (Key :type "Key Structure")))

(event `Key|I`
  (params (Key :type "Key Structure"))
  (bind _itemwidget (`self.ItemWidget`))
  ;[1 1 1] Menu
  (:`Pressed`
    (if (`self.IsPlayerMenuShow`)
      _
      (elif (`Widget.IsInViewport` _itemwidget)
        (`Widget.RemoveFromParent` _itemwidget)
        (else
          (`UserWidget.AddToViewport` _itemwidget 0)
          (`Widget.RemoveFromParent` (`self.SkillWidget`)))))))

(event `Key|A`
  (params (Key :type "Key Structure"))
  (bind _actorwidget (`self.ActorWidget`))
  ;[1 1 1] Menu
  (:`Pressed`
    (if (`self.IsPlayerMenuShow`)
      _
      (elif (`Widget.IsInViewport` _actorwidget)
        (`Widget.RemoveFromParent` _actorwidget)
        (else
          (`UserWidget.AddToViewport` _actorwidget 0)
          (`Widget.RemoveFromParent` (`self.SkillWidget`)))))))

(event `Key|T`
  (params (Key :type "Key Structure"))
  (bind _skillwidget (`self.SkillWidget`))
  ;[1 1 1] Menu
  (:`Pressed`
    (if (`self.IsPlayerMenuShow`)
      _
      (elif (`Widget.IsInViewport` _skillwidget)
        (`Widget.RemoveFromParent` _skillwidget)
        (else
          (`UserWidget.AddToViewport` _skillwidget 0)
          (`Widget.RemoveFromParent` (`self.ActorWidget`))
          (`Widget.RemoveFromParent` (`self.ItemWidget`)))))))

(event `Key|Escape`
  (params (Key :type "Key Structure"))
  ;[1 1 1] Menu
)

(event `Key|Tab`
  (params (Key :type "Key Structure"))
  (bind _menuwidget (`self.MenuWidget`))
  ;[1 1 1] Menu
  (:`Pressed`
    (if (`Widget.IsInViewport` _menuwidget)
      (`Widget.RemoveFromParent` _menuwidget)
      (else
        (`UserWidget.AddToViewport` _menuwidget 0)
        (`Widget.RemoveFromParent` (`self.ActorWidget`))
        (`Widget.RemoveFromParent` (`self.ItemWidget`))
        (`Widget.RemoveFromParent` (`self.SkillWidget`))))))

(event `Key|MouseScrollUp`
  (params (Key :type "Key Structure"))
  (bind _cameraboom (`self.CameraBoom`))
  (bind _returnvalue (- (`SpringArmComponent.TargetArmLength` _cameraboom) 100.0))
  ;[1 1 1] Camera Boom
  (:`Pressed`
    (if (>= _returnvalue 600.0)
      (set `SpringArmComponent.TargetArmLength` _returnvalue _cameraboom))))

(event `Key|MouseScrollDown`
  (params (Key :type "Key Structure"))
  (bind _cameraboom (`self.CameraBoom`))
  (bind _returnvalue (+ (`SpringArmComponent.TargetArmLength` _cameraboom) 100.0))
  ;[1 1 1] Camera Boom
  (:`Pressed`
    (if (<= _returnvalue 1400.0)
      (set `SpringArmComponent.TargetArmLength` _returnvalue _cameraboom))))

(event `Key|One`
  (params (Key :type "Key Structure"))
  (bind _returnvalue (`AbilitySystemBlueprintLibrary.GetAbilitySystemComponent` self))
  (:`Pressed`
    (if (>= (`AbilitySystemComponent.GetGameplayEffectCount` _returnvalue "/Game/Blueprints/Character/Abilitys/GE_RecoverBuff.GE_RecoverBuff_C" null true) 1)
      (`AbilitySystemComponent.RemoveActiveGameplayEffectBySourceEffect` _returnvalue "/Game/Blueprints/Character/Abilitys/GE_RecoverBuff.GE_RecoverBuff_C" null -1)
      (else
        (`AbilitySystemComponent.BP_ApplyGameplayEffectToSelf` _returnvalue "/Game/Blueprints/Character/Abilitys/GE_RecoverBuff.GE_RecoverBuff_C" 1.0 (`AbilitySystemComponent.MakeEffectContext` _returnvalue))))))

(event `Key|RightMouseButton`
  (params (Key :type "Key Structure"))
  (:`Pressed`
    (`self.TryActivateAbility` "/Game/Blueprints/Character/Abilitys/GA_Melee.GA_Melee_C")))

(event `Key|Q`
  (params (Key :type "Key Structure"))
  (:`Pressed`
    (`self.TryActivateAbility` "/Game/Blueprints/Character/Abilitys/GA_FireBall.GA_FireBall_C")))

(event `self.OnHealthChanged`
  (params (DeltaValue :type "Float (single-precision)") (EventTags :type "GameplayTagContainer Structure (by ref)"))
  (`KismetSystemLibrary.PrintString` (`KismetStringLibrary.Conv_DoubleToString` (`self.GetHealth`))))

(fn `AddExperience`
  (params (NewParam :type Integer))
  (locals (LocalExperience :type Integer))
  (bind _output_get (set `local.LocalExperience` (- (`self.GetCharacterExperience`) NewParam)))
  (if (<= _output_get 0)
    (bind _returnvalue (`self.SetCharacterLevel` (+ (`self.GetCharacterLevel`) 1)))
    (bind _returnvalue_2 (`self.SetMaxCharacterExperience` (* _returnvalue 100)))
    (`self.SetCharacterExperience` _returnvalue_2)
    (`self.SetCharacterExperience` (+ (`self.GetCharacterExperience`) (`local.LocalExperience`)))
    (else
      (`self.SetCharacterExperience` (`local.LocalExperience`)))))

(fn `AttachCurrentWeapon`
  (params (WeaponData :type "UniqueData Structure"))
  (bind _returnvalue (`|SpawnActorFromClass` "/Game/Blueprints/Character/Skill/WeaponActor.WeaponActor_C" (`KismetMathLibrary.MakeTransform` (0.0 0.0 0.0) (struct :`Roll` -90.0)) "Undefined" "OverrideRootScale" null null))
  (bind _output_get (set `self.currentWeapon` _returnvalue))
  (set `/Game/Blueprints/Character/Skill/WeaponActor.WeaponData` WeaponData _output_get)
  (`self.K2_AttachToComponent` (`self.currentWeapon`) (`self.Mesh`) "b_MF_Weapon_R_Socket" "KeepRelative" "KeepRelative" "KeepRelative" true))

(fn `CreateMenu`
  (`|ExecutionSequence`
    (:`then_0`
      (bind _returnvalue (`|CreateWidget` "/Game/Blueprints/WidgetBP/Character/HeroSkill.HeroSkill_C" (`GameplayStatics.GetPlayerController` 0)))
      (set `self.SkillWidget` _returnvalue))
    (:`then_1`
      (bind _returnvalue_2 (`|CreateWidget` "/Game/Blueprints/WidgetBP/Character/HeroEquipment.HeroEquipment_C" (`GameplayStatics.GetPlayerController` 0)))
      (set `self.ItemWidget` _returnvalue_2))
    (:`then_2`
      (bind _returnvalue_3 (`|CreateWidget` "/Game/Blueprints/WidgetBP/Character/HeroProperty.HeroProperty_C" (`GameplayStatics.GetPlayerController` 0)))
      (set `self.ActorWidget` _returnvalue_3))
    (:`then_3`
      (bind _returnvalue_4 (`|CreateWidget` "/Game/Blueprints/WidgetBP/Menu/PlayerMenu.PlayerMenu_C" (`GameplayStatics.GetPlayerController` 0)))
      (set `self.MenuWidget` _returnvalue_4))
    (:`then_4`
      (bind _returnvalue_5 (`|CreateWidget` "/Game/Blueprints/WidgetBP/Level/HUD.HUD_C" (`GameplayStatics.GetPlayerController` 0)))
      (bind _output_get (set `self.HUDWidget` _returnvalue_5))
      (`UserWidget.AddToViewport` _output_get 0))
    (:`then_5`
      (bind _returnvalue_6 (`|CreateWidget` "/Game/Blueprints/WidgetBP/Character/StoreHouse.StoreHouse_C" (`GameplayStatics.GetPlayerController` 0)))
      (set `self.StortWidget` _returnvalue_6))))

(fn `FireBall`
  (bind (_returnvalue_location _returnvalue_rotation) (`KismetMathLibrary.BreakTransform` (`SceneComponent.K2_GetComponentToWorld` (`self.Sphere`))))
  (`|SpawnActorFromClass` "/Game/Blueprints/Character/Skill/BP_FireBall.BP_FireBall_C" (`KismetMathLibrary.MakeTransform` _returnvalue_location _returnvalue_rotation) "AlwaysSpawn" "OverrideRootScale" null null))

(fn `GetAttackPowerA`
  (returns (NewPower :type "Float (double-precision)"))
  (`/Engine/EditorBlueprintResources/StandardMacros.IsValid` (`self.currentWeapon`)
    (:`Is Valid`
      (bind _asweapon_item (cast `WeaponItem` (`.Item` (break `UniqueData` (`/Game/Blueprints/Character/Skill/WeaponActor.WeaponData` (`self.currentWeapon`))))))
      (return (+ (`WeaponItem.MinDamage` _asweapon_item) (`self.GetAttackPower`))))
    (:`Is Not Valid`
      (return (`self.GetAttackPower`)))))

(fn `GetAttackSpeedA`
  (returns (NewSpeed :type "Float (double-precision)"))
  (`/Engine/EditorBlueprintResources/StandardMacros.IsValid` (`self.currentWeapon`)
    (:`Is Valid`
      (bind _asweapon_item (cast `WeaponItem` (`.Item` (break `UniqueData` (`/Game/Blueprints/Character/Skill/WeaponActor.WeaponData` (`self.currentWeapon`))))))
      (return (+ (`WeaponItem.Speed` _asweapon_item) (`self.GetAttackSpeed`))))
    (:`Is Not Valid`
      (return (`self.GetAttackSpeed`)))))

(fn `GetHealthA`
  (returns (NewHealth :type "Float (double-precision)"))
  (`/Engine/EditorBlueprintResources/StandardMacros.IsValid` (`self.currentWeapon`)
    (:`Is Valid`
      (return (+ (`.Health` (break `UniqueData` (`/Game/Blueprints/Character/Skill/WeaponActor.WeaponData` (`self.currentWeapon`)))) (`self.GetHealth`))))
    (:`Is Not Valid`
      (return (`self.GetHealth`)))))

(fn `GetMaxHealthA`
  (returns (NewMaxHealth :type "Float (double-precision)"))
  (`/Engine/EditorBlueprintResources/StandardMacros.IsValid` (`self.currentWeapon`)
    (:`Is Valid`
      (return (+ (`.Health` (break `UniqueData` (`/Game/Blueprints/Character/Skill/WeaponActor.WeaponData` (`self.currentWeapon`)))) (`self.GetMaxHealth`))))
    (:`Is Not Valid`
      (return (`self.GetMaxHealth`)))))

(fn `HideStoreWidget`
  (`Widget.RemoveFromParent` (`self.ItemWidget`))
  (`Widget.RemoveFromParent` (`self.StortWidget`)))

(fn `InitCharacter`
  (bind _mesh (`self.Mesh`))
  (bind _returnvalue (`|GetDataTableRow` "/Game/Blueprints/Character/Hero/SkeletalMeshData/HeroDataTable.HeroDataTable" (`self.HeroName`))
    (:`then`
      (bind (_mesh_2 _animblueprint) (break `/Game/Blueprints/Character/Hero/SkeletalMeshData/HeroStruct` _returnvalue))
      (`SkeletalMeshComponent.SetSkeletalMeshAsset` _mesh _mesh_2)
      (`SkeletalMeshComponent.SetAnimInstanceClass` _mesh _animblueprint))))

(fn `Pick Up Potion`
  (params (DataAsset :type "DiaBalShadowPrimaryDataAsset Object Reference"))
  (`/Game/Blueprints/WidgetBP/Character/HeroEquipment.AddItem` :`self` (`self.ItemWidget`) :`AssertData` DataAsset :`IsPickUp` true))

(fn `Pick Up Weapon`
  (params (UniqueData :type "UniqueData Structure"))
  (`/Game/Blueprints/WidgetBP/Character/HeroEquipment.AddItem` (`self.ItemWidget`) UniqueData null true)
  (`self.Remove Current Weapon`)
  (`self.AttachCurrentWeapon` UniqueData))

(fn `Remove Current Weapon`
  (`/Engine/EditorBlueprintResources/StandardMacros.IsValid` (`self.currentWeapon`)
    (:`Is Valid`
      (`self.K2_DestroyActor` (`self.currentWeapon`)))))

(fn `ShowStoreWidget`
  (if (not (`self.IsPlayerMenuShow`))
    (`UserWidget.AddToViewport` (`self.ItemWidget`) 0)
    (`UserWidget.AddToViewport` (`self.StortWidget`) 0)
    (`Widget.RemoveFromParent` (`self.SkillWidget`))))

(fn `TryActivateAbility`
  (params (class :type "GameplayAbility Class Reference"))
  (`AbilitySystemComponent.TryActivateAbilityByClass` (`AbilitySystemBlueprintLibrary.GetAbilitySystemComponent` self) class true))

(fn `UserConstructionScript`
  (bind _asbp_game_instance (cast `/Game/Blueprints/Character/BP_GameInstance` (`GameplayStatics.GetGameInstance`)))
  (bind _returnvalue (`DiaBalShadowGameInstance.GetDefaultCharacter` _asbp_game_instance))
  (bind (_name _heroname) (break `CharacterData` _returnvalue))
  (set `self.PlayerName` _name)
  (bind _output_get (set `self.HeroName` _heroname))
  (bind _returnvalue_2 (`|GetDataTableRow` "/Game/Blueprints/Character/Hero/StateData/StateDataTable.StateDataTable" _output_get)
    (:`then`
      (`KismetArrayLibrary.Array_Add` (`self.PassiveGameplayEffects`) (`.State_2_DBE9DBC441E1146BD92872BC7E70D92D` (break `/Game/Blueprints/Character/Hero/StateData/StateStruct` _returnvalue_2))))))