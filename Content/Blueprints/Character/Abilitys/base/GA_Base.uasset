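; GA_Base is a base Gameplay Ability that plays a skill montage and applies an effect to the target it reports.
; On activation, a two-stage data table lookup picks the montage by player 0's hero name, then SkillName.
; After committing cost and cooldown, it waits for Event.Montage events during playback.
; An event ends the ability and applies the effect container to the target's ability system; montage completion, blend-out, interruption or cancellation just ends it.
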(event `self.K2_ActivateAbility`
  (`self.Get Skill `)
  (bind _returnvalue (`self.K2_CommitAbility`)) ; Handles any costs or cooldowns
  (if _returnvalue
    (bind (_asynctaskproxy _eventtag _eventdata) (`DiaBalShadowAbilityTask_PlayMontageAndWaitForEvent.PlayMontageAndWaitForEvent` "None" (`self.AnimMontage`) (struct :`GameplayTags` (struct :`(TagName` "Event.Montage"))))
      (:`OnCompleted`
        (`self.K2_EndAbility` :!label _label))
      (:`OnBlendOut`
        (goto _label))
      (:`OnInterrupted`
        (goto _label))
      (:`OnCancelled`
        (goto _label))
      (:`EventReceived`
        (`self.K2_EndAbility`)
        (`self.ApplyEffectContainer` (`self.Effect`) (`AbilitySystemBlueprintLibrary.GetAbilitySystemComponent` (`.Target` (break `GameplayEventData` _eventdata))))))))

(fn `Get Skill `
  (bind _asbp_character (cast `/Game/Blueprints/Character/BP_Character` (`GameplayStatics.GetPlayerCharacter` 0)))
  (bind _returnvalue (`|GetDataTableRow` "/Game/Blueprints/Character/Hero/SkillData/SkillDataTable.SkillDataTable" (`/Game/Blueprints/Character/BP_Character.HeroName` _asbp_character))
    (:`then`
      (bind _returnvalue_2 (`|GetDataTableRow` (`.DataTable_2_D20CB76043D8E0B99D487A91525B861F` (break `/Game/Blueprints/Character/Hero/SkillData/SkillDataTableStruct` _returnvalue)) (`self.SkillName`))
        (:`then`
          (set `self.AnimMontage` (`.Skill_8_A31BCF5B4CF01D1060184DB903FEA270` (break `/Game/Blueprints/Character/Hero/SkillData/SkillStruct` _returnvalue_2))))))))