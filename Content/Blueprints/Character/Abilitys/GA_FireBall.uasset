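; GA_FireBall is a fireball gameplay ability that turns the player character toward the mouse cursor when activated.
; It traces under the cursor on the Visibility channel and applies only the yaw of the look-at rotation to player 0's character.
; The parent ability's activation runs only if the trace hits and the rotation succeeds, leaving the rest of the ability's behavior to the parent class.
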(event `self.K2_ActivateAbility`
  (bind _returnvalue (`GameplayStatics.GetPlayerCharacter` 0))
  (bind (_hitresult _returnvalue_2) (`PlayerController.GetHitResultUnderCursorByChannel` (`GameplayStatics.GetPlayerController` 0) "TraceTypeQuery1" true))
  (bind (_returnvalue_roll _returnvalue_pitch _returnvalue_yaw) (`KismetMathLibrary.BreakRotator` (`KismetMathLibrary.FindLookAtRotation` (`Actor.K2_GetActorLocation` _returnvalue) (`.Location` (`GameplayStatics.BreakHitResult` _hitresult)))))
  (if _returnvalue_2
    (bind _returnvalue_3 (`Actor.K2_SetActorRotation` _returnvalue (`KismetMathLibrary.MakeRotator` 0.0 0.0 _returnvalue_yaw) false))
    (if _returnvalue_3
      (`parent.K2_ActivateAbility`))))