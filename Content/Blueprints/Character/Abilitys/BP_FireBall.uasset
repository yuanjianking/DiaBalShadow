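; BP_FireBall is a short-lived fireball ability actor that deals its effect to whatever character it overlaps.
; A one-second timer destroys it if nothing is touched first.
; Any overlap spawns a particle burst at the other actor and destroys the fireball.
; If that actor is a DiaBalShadowCharacterBase, its own Ability System Component applies GE_FireBall to itself, so no instigator is passed from the fireball.
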(event `self.ReceiveBeginPlay`
  (`KismetSystemLibrary.K2_SetTimerDelegate` (delegate `自定义事件`) 1.0)
  (add `self.OnActorBeginOverlap` (delegate `OnActorBeginOverlap_Event`)))

(event `自定义事件`
  (`self.K2_DestroyActor`))

(event `OnActorBeginOverlap_Event` :!signature `self.OnActorBeginOverlap`
  (params (OverlappedActor :type "Actor Object Reference") (OtherActor :type "Actor Object Reference"))
  (bind (_returnvalue_location _returnvalue_rotation) (`KismetMathLibrary.BreakTransform` (`self.GetTransform` OtherActor)))
  (`GameplayStatics.SpawnEmitterAtLocation` "/Engine/Tutorial/SubEditors/TutorialAssets/TutorialParticleSystem.TutorialParticleSystem" _returnvalue_location _returnvalue_rotation)
  (`self.K2_DestroyActor`)
  (bind _asdia_bal_shadow_character_base (cast `DiaBalShadowCharacterBase` OtherActor))
  (bind _returnvalue (`AbilitySystemBlueprintLibrary.GetAbilitySystemComponent` _asdia_bal_shadow_character_base))
  (`AbilitySystemComponent.BP_ApplyGameplayEffectToTarget` _returnvalue "/Game/Blueprints/Character/Abilitys/GE_FireBall.GE_FireBall_C" _returnvalue 1.0 (`AbilitySystemComponent.MakeEffectContext` _returnvalue)))

(fn `UserConstructionScript`)