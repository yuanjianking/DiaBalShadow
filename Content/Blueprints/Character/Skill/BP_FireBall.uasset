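; Fireball skill actor that reports enemy hits back to the ability of the character that fired it.
; It destroys itself after a short timer or on its first actor overlap, spawning an impact particle at the overlapped actor's location.
; If that actor is a DiaBalShadowEnemyCharacter, it sends the Event.Montage.fireball gameplay event to its instigator with the enemy as target.
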(event `self.ReceiveBeginPlay`
  (`KismetSystemLibrary.K2_SetTimerDelegate` (delegate `自定义事件`) 1.0)
  (add `self.OnActorBeginOverlap` (delegate `OnActorBeginOverlap_Event`)))

(event `自定义事件`
  (`self.K2_DestroyActor`))

(event `OnActorBeginOverlap_Event` :!signature `self.OnActorBeginOverlap`
  (params (OverlappedActor :type "Actor Object Reference") (OtherActor :type "Actor Object Reference"))
  (bind _returnvalue (`self.GetInstigator`))
  (bind (_returnvalue_location _returnvalue_rotation) (`KismetMathLibrary.BreakTransform` (`self.GetTransform` OtherActor)))
  (`GameplayStatics.SpawnEmitterAtLocation` "/Game/InfinityBladeEffects/Effects/FX_Monsters/FX_Monster_Chicken/P_ChickenMaster_Melee_Imp_01.P_ChickenMaster_Melee_Imp_01" _returnvalue_location _returnvalue_rotation (1.0 1.0 1.0) true "AutoRelease")
  (`self.K2_DestroyActor`)
  (bind _asdia_bal_shadow_enemy_character (cast `DiaBalShadowEnemyCharacter` OtherActor))
  (`AbilitySystemBlueprintLibrary.SendGameplayEventToActor` _returnvalue (struct :`TagName` "Event.Montage.fireball") (make `GameplayEventData` (struct) _returnvalue _asdia_bal_shadow_enemy_character)) ; Pass hit information back to ability
)

(fn `UserConstructionScript`)