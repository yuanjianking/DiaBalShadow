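; Menu game mode for character creation and selection, swapping the create and choice widgets and blending the view between their two cameras.
; Init stores both cameras, builds the widgets and opens the create menu.
; That menu loads the GameInstance's default hero, applying its data-table mesh and AnimBlueprint to CreateCamera, which doubles as a HeroBase.
; Axis-driven helpers yaw a target or slide it along Y within fixed bounds.
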(event `self.ReceiveBeginPlay`
  (`self.InitInput`))

(fn `GetDefaultCharater`
  (returns (Charater :type "CharacterData Structure"))
  (bind _asbp_game_instance (cast `/Game/Blueprints/Character/BP_GameInstance` (`GameplayStatics.GetGameInstance`)))
  (bind _returnvalue (`DiaBalShadowGameInstance.GetDefaultCharacter` _asbp_game_instance))
  (return _returnvalue))

(fn `Init`
  (params (CreateCamera :type "Actor Object Reference") (ChoiceCamera :type "Actor Object Reference"))
  (set `self.CreateCamera` CreateCamera)
  (set `self.ChoiceCamera` ChoiceCamera)
  (bind _returnvalue (`|CreateWidget` "/Game/Blueprints/WidgetBP/Menu/CreateCharater.CreateCharater_C"))
  (set `self.CreateCharaterWidget` _returnvalue)
  (bind _returnvalue_2 (`|CreateWidget` "/Game/Blueprints/WidgetBP/Menu/ChoiceCharacter.ChoiceCharacter_C"))
  (set `self.ChoiceCharaterWidget` _returnvalue_2)
  (`self.ShowCreateMenu`))

(fn `LoadCharacter`
  (`/Game/Blueprints/WidgetBP/Menu/CreateCharater.AddCharacter` (`self.CreateCharaterWidget`))
  (bind _charater (`self.GetDefaultCharater`))
  (bind _returnvalue (`|GetDataTableRow` "/Game/Blueprints/Character/Hero/SkeletalMeshData/HeroDataTable.HeroDataTable" (`KismetStringLibrary.Conv_StringToName` (`.HeroName` (break `CharacterData` _charater))))
    (:`then`
      (bind _ashero_base (cast `/Game/Blueprints/Character/Hero/SkeletalMesh/HeroBase` (`self.CreateCamera`)))
      (bind (_mesh _animblueprint) (break `/Game/Blueprints/Character/Hero/SkeletalMeshData/HeroStruct` _returnvalue))
      (`/Game/Blueprints/Character/Hero/SkeletalMesh/HeroBase.SetMesh` _ashero_base _mesh _animblueprint))
    (:`RowNotFound`
      (bind _ashero_base_2 (cast `/Game/Blueprints/Character/Hero/SkeletalMesh/HeroBase` (`self.CreateCamera`)))
      (`/Game/Blueprints/Character/Hero/SkeletalMesh/HeroBase.SetMesh` _ashero_base_2 null null))))

(fn `MoveCamera`
  (params (`目标` :type "Actor Object Reference"))
  (bind (_returnvalue_x _returnvalue_y _returnvalue_z) (`KismetMathLibrary.BreakVector` (+ (`self.K2_GetActorLocation` `目标`) (`KismetMathLibrary.MakeVector` 0.0 (* (* (`self.GetInputAxisKeyValue`) -1.0) 10.0)))))
  (if (not (or (> _returnvalue_y 800.0) (< _returnvalue_y -600.0)))
    (`self.K2_SetActorLocation` `目标` (`KismetMathLibrary.MakeVector` _returnvalue_x _returnvalue_y _returnvalue_z) true false)))

(fn `RotationCamera`
  (params (`目标` :type "SceneComponent Object Reference"))
  (`SceneComponent.K2_AddRelativeRotation` `目标` (`KismetMathLibrary.MakeRotator` 0.0 0.0 (* (* (`self.GetInputAxisKeyValue`) -1.0) 10.0)) false false))

(fn `ShowChoiceMenu`
  (`Widget.RemoveFromParent` (`self.CreateCharaterWidget`))
  (`UserWidget.AddToViewport` (`self.ChoiceCharaterWidget`) 0)
  (`self.SwitchCamera` (`self.ChoiceCamera`)))

(fn `ShowCreateMenu`
  (`Widget.RemoveFromParent` (`self.ChoiceCharaterWidget`))
  (`UserWidget.AddToViewport` (`self.CreateCharaterWidget`) 0)
  (`self.SwitchCamera` (`self.CreateCamera`))
  (`self.LoadCharacter`))

(fn `SwitchCamera`
  (params (NewViewTarget :type "Actor Object Reference"))
  (`PlayerController.SetViewTargetWithBlend` (`GameplayStatics.GetPlayerController` 0) NewViewTarget 0.0 "VTBlend_EaseInOut" 0.0 false))

(fn `UserConstructionScript`)