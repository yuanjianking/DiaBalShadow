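; Base enemy Blueprint with a health widget, a melee attack and death rewards.
; On BeginPlay it registers itself with its EnemyHealth widget, and MeleeAttack activates the GA_EnemyMelee ability through the Gameplay Ability System.
; When health reaches zero it flags itself dead, grants the player experience, spawns offset health and mana pickups, then destroys itself after a short delay.
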(event `self.ReceiveBeginPlay`
  (bind _asenemy_health (cast `/Game/Blueprints/WidgetBP/Enemy/EnemyHealth` (`WidgetComponent.GetWidget` (`self.Health`))))
  (set `/Game/Blueprints/WidgetBP/Enemy/EnemyHealth.Enemy` self _asenemy_health))

(event `self.OnHealthChanged`
  (params (DeltaValue :type "Float (single-precision)") (EventTags :type "GameplayTagContainer Structure (by ref)"))
  (bind _returnvalue (`self.GetTransform`))
  (bind _returnvalue_2 (`self.GetTransform`))
  (if (<= (`self.GetHealth`) 0.0)
    (set `self.IsDead` true)
    (bind _asbp_character (cast `/Game/Blueprints/Character/BP_Character` (`GameplayStatics.GetPlayerCharacter` 0)))
    (`/Game/Blueprints/Character/BP_Character.AddExperience` _asbp_character 70)
    (`|SpawnActorFromClass` "/Game/Assets/Pickups/PotionPickups/BP_Pickup_Health.BP_Pickup_Health_C" (`KismetMathLibrary.MakeTransform` (`KismetMathLibrary.MakeVector` (+ (.x (.location _returnvalue)) 200.0) (+ (.y (.location _returnvalue)) 200.0))) "AlwaysSpawn" "OverrideRootScale" null null)
    (`|SpawnActorFromClass` "/Game/Assets/Pickups/PotionPickups/BP_Pickup_Mana.BP_Pickup_Mana_C" (`KismetMathLibrary.MakeTransform` (`KismetMathLibrary.MakeVector` (+ (.x (.location _returnvalue_2)) 300.0) (+ (.y (.location _returnvalue_2)) 300.0))) "AlwaysSpawn" "OverrideRootScale" null null)
    (`KismetSystemLibrary.Delay` 1.5)
    (`self.K2_DestroyActor`)))

(fn `MeleeAttack`
  (`AbilitySystemComponent.TryActivateAbilityByClass` (`AbilitySystemBlueprintLibrary.GetAbilitySystemComponent` self) "/Game/Blueprints/Enemy/Abilitys/GA_EnemyMelee.GA_EnemyMelee_C" true))

(fn `UserConstructionScript`)