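; BP_PotionPickup is a potion pickup that a BP_Character collects by touching it.
; On BeginPlay it sets the text of its Pickup widget to the item name from its DataAssert variable.
; When a BP_Character overlaps the Sphere, it passes DataAssert to that character's PickUpPotion and destroys itself.
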(event `self.ReceiveBeginPlay`
  (bind _aspickup (cast `/Game/Blueprints/WidgetBP/Assets/Pickup` (`WidgetComponent.GetUserWidgetObject` (`self.Widget`))))
  (`/Game/Blueprints/WidgetBP/Assets/Pickup.SetText` _aspickup (`DiaBalShadowPrimaryDataAsset.ItemName` (`self.DataAssert`))))

(event `self.Sphere.OnComponentBeginOverlap`
  (params (OverlappedComponent :type "PrimitiveComponent Object Reference") (OtherActor :type "Actor Object Reference") (OtherComp :type "PrimitiveComponent Object Reference") (OtherBodyIndex :type Integer) (bFromSweep :type Boolean) (SweepResult :type "HitResult Structure (by ref)"))
  (bind _asbp_character (cast `/Game/Blueprints/Character/BP_Character` OtherActor))
  (`/Game/Blueprints/Character/BP_Character.Pick Up Potion` _asbp_character (`self.DataAssert`))
  (`self.K2_DestroyActor`))

(fn `UserConstructionScript`)